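; BP_ControlArea is an actor in the drive level that sends the player into BuildingLevel through a trigger.
; On BeginPlay it caches the first actor tagged "Portal" as a BP_Portal reference, which this graph does not use further.
; When a BP_ThirdPersonCharacter overlaps EnterBuildingTrigger, the EnterBuilding event opens BuildingLevel by name, with debug prints along the way.
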(event OnComponentBeginOverlap(EnterBuildingTrigger)
  (params (OverlappedComponent :type Primitive%20Component%20Object%20Reference) (OtherActor :type Actor%20Object%20Reference) (OtherComp :type Primitive%20Component%20Object%20Reference) (OtherBodyIndex :type Integer) (bFromSweep :type Boolean) (SweepResult :type Hit%20Result%20Structure%20%28by%20ref%29))
  (Development|PrintString "포탈 충돌 감지")
  (Utilities|Casting|CastToBP_ThirdPersonCharacter OtherActor)
  (CallFunction|EnterBuilding))

(event Custom|EnterBuilding
  (Development|PrintString "다음 레벨 호출")
  (Game|OpenLevel(byName) "BuildingLevel"))

(event EventBeginPlay
  (bind _outactors (Actor|GetAllActorswithTag "Portal"))
  (bind _asbp_portal (Utilities|Casting|CastToBP_Portal (Utilities|Array|Get(acopy) _outactors)))
  (Variables|Default|SetBP_PortalRef _asbp_portal))

(fn ConstructionScript)